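; BP_Sun_Rotation turns the referenced sun actor each frame to move the sun across the sky at the game's speed.
; It reads game speed from BP_RTS_GameState on BeginPlay and binds to its speed-control event for later changes.
; Tick feeds delta time and speed through SetGameTime, scales the result into a local pitch rotation, then updates the sky sphere's sun direction.
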(event `self.ReceiveBeginPlay`
  (set `self.Game_State_Ref` (cast `/Game/MY_Scripts/Blueprints/Game_Settings/BP_RTS_GameState` (`GameplayStatics.GetGameState`) :!pure true))
  (add `/Game/MY_Scripts/Blueprints/Game_Settings/BP_RTS_GameState.Game_Speed_Control` (`self.Game_State_Ref`) (`|CreateDelegate` :!event `GetGameSpeed`))
  (bind _game_speed (`/Game/MY_Scripts/Blueprints/Game_Settings/BP_RTS_GameState.Get_Game_Speed` (`self.Game_State_Ref`)))
  (set `self.Game_Speed` _game_speed))

(event `GetGameSpeed`
  (params (Game_Speed :type "Float (double-precision)"))
  (set `self.Game_Speed` Game_Speed))

(event `self.ReceiveTick`
  (params (DeltaSeconds :type "Float (single-precision)"))
  (`self.K2_AddActorLocalRotation` (`self.Sun_Ref`) (`KismetMathLibrary.MakeRotator` 0.0 (* (/ (/ (`/Game/MY_Scripts/Blueprints/Libraries/BP_RTS_FunctionLib.Set_Game_Time` DeltaSeconds (`self.Game_Speed`) (`self.Game_Time`)) 1.5) 6.0) 90.0)) false false)
  (`/Engine/EngineSky/BP_Sky_Sphere.UpdateSunDirection` (`self.Sky_Sphere_Ref`)))

(fn `UserConstructionScript`)