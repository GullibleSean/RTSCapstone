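; RTS game state that runs the in-game clock and calendar.
; Tick advances GameTime by GameSpeed, derives time and date with day, month and year rollover, then pushes both to the player controller's HUD and debug prints.
; Tick also rebuilds the list of all units through GetAllActorsOfClass every frame.
; UpdateGameSpeed writes the scaled default speed into GameTime, not GameSpeed, and passes it to CallGameSpeedControl.
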(event `self.ReceiveBeginPlay`
  (`|ExecutionSequence`
    (:`then_0`
      (`self.ReferenceCast`))
    (:`then_1`
      ;[1 1 1] Initial Game Time
      (set `self.Game_Time` (+ (`KismetMathLibrary.Conv_IntToDouble` (`self.Hours`)) (/ (`KismetMathLibrary.Conv_IntToDouble` (`self.Minutes`)) 60.0) (/ (`KismetMathLibrary.Conv_IntToDouble` (`self.Seconds`)) 3600.0)))
      (set `self.Game_Date` (`|MakeArray` (`self.Day`) (`self.Month`) (`self.Year`))))
    (:`then_2`
      (set `self.Game_Speed` (`self.Default_Game_Speed`)))))

(event `self.ReceiveTick`
  (params (DeltaSeconds :type "Float (single-precision)"))
  (bind (_game_time _day_count) (`/Game/MY_Scripts/Blueprints/Libraries/BP_RTS_FunctionLib.Set_Game_Time` DeltaSeconds (`self.Game_Speed`) (`self.Game_Time`)))
  (set `self.Game_Time` _game_time)
  (set `self.Day_Counter` _day_count)
  (`self.Set_Clock`)
  (`self.Set_Calendar`)
  (`self.GetAllUnits`))

(event `/Game/MY_Scripts/Blueprints/Libraries/BPI_RTS_Time_Interface.Update_Game_Speed`
  (params (Speed_Multiplier :type "Float (single-precision)"))
  (bind _output_get (set `self.Speed_Multiplier` Speed_Multiplier))
  (bind _output_get_2 (set `self.Game_Time` (* _output_get (`self.Default_Game_Speed`))))
  (`self.Game_Speed_Control` _output_get_2))

(fn `Get_Game_Speed`
  (returns (Game_Speed :type "Float (double-precision)"))
  (return (`self.Game_Speed`)))

(fn `GetAllUnits`
  (returns (UnitOut :type "Array of /Game/MY_Scripts/Blueprints/Units/BP_RTS_Unit_Master Object Reference"))
  (bind _outactors (`GameplayStatics.GetAllActorsOfClass` "/Game/MY_Scripts/Blueprints/Units/BP_RTS_Unit_Master.BP_RTS_Unit_Master_C"))
  (bind _output_get (set `self.ListOfAllUnits` _outactors))
  (return _output_get))

(fn `Set_Calendar`
  (bind _output_get (set `self.Day` (+ (`self.Day`) (`self.Day_Counter`))))
  (if (> _output_get (`KismetMathLibrary.DaysInMonth` (`self.Year`) (`self.Month`)))
    (set `self.Day` 1)
    (set `self.Month` (+ (`self.Month`) 1)))
  (if (> (`self.Month`) 12)
    (set `self.Month` 1)
    (set `self.Year` (+ (`self.Year`) 1)))
  (bind _output_get_2 (set `self.Game_Date` (`|MakeArray` (`self.Day`) (`self.Month`) (`self.Year`))))
  (message `/Game/MY_Scripts/Blueprints/Libraries/BPI_RTS_Time_Interface.Set_Game_Calendar` (`/Game/MY_Scripts/Blueprints/Player/BP_RTS_PlayerController.HUDMainGameRef` (`self.Controller_Reference`)) _output_get_2)
  (`KismetSystemLibrary.PrintString` (`KismetStringLibrary.BuildString_Int` (`KismetStringLibrary.BuildString_Int` (`KismetStringLibrary.Conv_IntToString` (`|GetArrayItem` _output_get_2)) "/ " (`|GetArrayItem` _output_get_2 1)) "/ " (`|GetArrayItem` _output_get_2 2))))

(fn `Set_Clock`
  (bind (_remainder _returnvalue) (`KismetMathLibrary.FMod` (* (`self.Game_Time`) 3600.0) 60.0))
  (bind (_remainder_2 _returnvalue_2) (`KismetMathLibrary.FMod` (`KismetMathLibrary.Conv_IntToDouble` _returnvalue) 60.0))
  (set `self.Seconds` (`KismetMathLibrary.FFloor` _remainder))
  (set `self.Minutes` (`KismetMathLibrary.FFloor` _remainder_2))
  (set `self.Hours` (`KismetMathLibrary.FFloor` (`KismetMathLibrary.FMod` (`KismetMathLibrary.Conv_IntToDouble` _returnvalue_2) 24.0)))
  (bind _output_get (set `self.Game_Date` (`|MakeArray` (`self.Seconds`) (`self.Minutes`) (`self.Hours`))))
  (message `/Game/MY_Scripts/Blueprints/Libraries/BPI_RTS_Time_Interface.Set_Game_Clock` (`/Game/MY_Scripts/Blueprints/Player/BP_RTS_PlayerController.HUDMainGameRef` (`self.Controller_Reference`)) _output_get)
  (`KismetSystemLibrary.PrintString` (`KismetStringLibrary.BuildString_Int` (`KismetStringLibrary.BuildString_Int` (`KismetStringLibrary.Conv_IntToString` (`|GetArrayItem` _output_get 2)) ": " (`|GetArrayItem` _output_get 1)) ": " (`|GetArrayItem` _output_get))))

(fn `Set_Game_Calendar`
  (params (Game_Date :type "Array of Integer (by ref)"))
  (returns (Success :type Boolean))
  (return false))

(fn `Set_Game_Clock`
  (params (Game_Time :type "Array of Integer (by ref)"))
  (returns (Success :type Boolean))
  (return false))

(fn `UserConstructionScript`)