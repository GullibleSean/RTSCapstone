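; BP_Resource_Master is a resource actor, named as the master Blueprint, that sets up its amount and appearance in the Construction Script.
; An optionally randomized resource level selects a multiplier that scales the base amount into CurrentResources.
; Optional flags then randomize the mesh's scale independently per axis and its yaw for visual variety.
; The event graph holds only disabled placeholder events, so it has no runtime logic.
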(fn `UserConstructionScript`
  (bind _returnvalue (`KismetMathLibrary.RandomFloatInRange` (`self.Min_Mesh_Size`) (`self.Max_Mesh_Size`)))
  (if (`self.Is_Random_Level`)
    (bind _output_get (set `self.E_Resource_Level` (cast `/Game/MY_Scripts/Blueprints/Enums/E_Resource_Level` (`KismetMathLibrary.Conv_IntToByte` (`KismetMathLibrary.RandomIntegerInRange` 1 6))))))
  (switch `/Game/MY_Scripts/Blueprints/Enums/E_Resource_Level` _output_get
    (:`NewEnumerator1`
      (set `self.Resource_Modifier` 1.0))
    (:`NewEnumerator2`
      (set `self.Resource_Modifier` 1.2))
    (:`NewEnumerator3`
      (set `self.Resource_Modifier` 1.4))
    (:`NewEnumerator4`
      (set `self.Resource_Modifier` 1.6))
    (:`NewEnumerator5`
      (set `self.Resource_Modifier` 1.8))
    (:`NewEnumerator6`
      (set `self.Resource_Modifier` 2.0)))
  (set `self.Current_Resources` (* (`self.Base_Resource_Amount`) (`self.Resource_Modifier`)))
  (if (`self.Is_Random_Size`)
    (`SceneComponent.SetWorldScale3D` (`self.ResourceMesh`) (`KismetMathLibrary.MakeVector` _returnvalue _returnvalue _returnvalue)))
  (if (`self.Is_Random_Rotated`)
    (`SceneComponent.K2_SetWorldRotation` (`self.ResourceMesh`) (`KismetMathLibrary.MakeRotator` 0.0 0.0 (`KismetMathLibrary.RandomFloatInRange` 0.0 360.0)) false false)))