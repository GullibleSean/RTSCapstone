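; Spawn volume that scatters resource actors at random points within its bounds for the RTS, on BeginPlay, on a looping timer, or both.
; Box traces place each actor only on Landscape hits, but the running total counts every requested spawn and caps timed spawning.
; RespawnTime follows pause, game speed, custom or combined settings using GameState speed.
; Tick recalculates it without restarting the timer.
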(event `self.ReceiveBeginPlay`
  (`|ExecutionSequence`
    (:`then_0`
      (`self.ReferenceCasts`))
    (:`then_1`
      (add `/Game/MY_Scripts/Blueprints/Game_Settings/BP_RTS_GameState.Game_Speed_Control` (`self.BP_RTS_GameState`) (`|CreateDelegate` :!event `GetGameSpeed`))
      (bind _game_speed (`/Game/MY_Scripts/Blueprints/Game_Settings/BP_RTS_GameState.Get_Game_Speed` (`self.BP_RTS_GameState`)))
      (set `self.Game_Speed` _game_speed)
      (`self.Set_Respawn_Timer`))
    (:`then_2`
      (if (`self.Is_Spawned_Begin_Play`)
        (`self.Spawn_Resource` (`self.Resource_Ref`) (`self.Number_of_Resources_Spawn`))
        (set `self.Total_Number_Spawned` (+ (`self.Number_of_Resources_Spawn`) (`self.Total_Number_Spawned`))))
      (if (`self.Is_Spawned_On_Timer`)
        (`KismetSystemLibrary.K2_SetTimerDelegate` (`|CreateDelegate` :!event `SpawnResourcesOnTimer`) (`self.Respawn_Time`) true)))))

(event `GetGameSpeed`
  (params (Game_Speed :type "Float (double-precision)"))
  (set `self.Game_Speed` Game_Speed))

(event `self.ReceiveTick`
  (params (DeltaSeconds :type "Float (single-precision)"))
  (`self.Set_Respawn_Timer`))

(event `SpawnResourcesOnTimer`
  (if (and (`self.Is_Spawned_On_Timer`) (< (`self.Total_Number_Spawned`) (`self.Max_Resources_Spawned`)))
    (`self.Spawn_Resource` (`self.Resource_Ref`) (`self.Number_of_Resources_Spawn`))
    (set `self.Total_Number_Spawned` (+ (`self.Number_of_Resources_Spawn`) (`self.Total_Number_Spawned`)))))

(fn `Add_Spawned_Resources_To_Total_Spawned`
  (set `self.Total_Number_Spawned` (+ (`self.Number_of_Resources_Spawn`) (`self.Total_Number_Spawned`))))

(fn `Check_Spawn_Timer_And_Total_Spawned`
  (if (and (`self.Is_Spawned_On_Timer`) (< (`self.Total_Number_Spawned`) (`self.Max_Resources_Spawned`)))
    _))

(fn `Set_Respawn_Timer`
  (returns (Respawn_Timer :type "Float (double-precision)"))
  (switch `/Game/MY_Scripts/Blueprints/Enums/E_Respawn_Timer` (`self.Time_Setting`)
    (:`NewEnumerator1`
      (set `self.Respawn_Time` 0.0))
    (:`NewEnumerator2`
      (set `self.Respawn_Time` (`self.Game_Speed`)))
    (:`NewEnumerator3`
      (set `self.Respawn_Time` (`self.User_Respawn_Timer`)))
    (:`NewEnumerator4`
      (set `self.Respawn_Time` (* (`self.User_Respawn_Timer`) (`self.Game_Speed`)))))
  (return (`self.Respawn_Time`)))

(fn `Spawn_Resource`
  (params (Resource :type "/Game/MY_Scripts/Blueprints/Resources/BP_Resource_Master Class Reference") (Spawn_Amount :type Integer))
  (locals (Resource_Ref_Local :type "/Game/MY_Scripts/Blueprints/Resources/BP_Resource_Master Class Reference") (Spawn_Amount_Local :type Integer))
  (bind (_origin _boxextent) (`self.GetActorBounds` false))
  (bind _x (.x _boxextent))
  (bind _y (.y _boxextent))
  (bind _returnvalue (+ _origin (`KismetMathLibrary.MakeVector` (`KismetMathLibrary.RandomFloatInRange` (- _x (* _x 2.0)) _x) (`KismetMathLibrary.RandomFloatInRange` (- _y (* _y 2.0)) _y) (.z _origin))))
  (set `local.Resource_Ref_Local` Resource)
  (set `local.Spawn_Amount_Local` Spawn_Amount)
  (for _ (range (+ (`local.Spawn_Amount_Local`) 1))
    (bind _outhit (`KismetSystemLibrary.BoxTraceSingle` (+ _returnvalue (0.0 0.0 200.0)) (0.0 0.0 0.0) (- _returnvalue (0.0 0.0 200.0)) (struct) "TraceTypeQuery1"))
    (bind (_bblockinghit _binitialoverlap _time _distance _location _impactpoint _normal _impactnormal _physmat _hitactor) (`GameplayStatics.BreakHitResult` _outhit))
    (if (== (`GameplayStatics.GetObjectClass` _hitactor) "/Script/Landscape.Landscape")
      (`|SpawnActorFromClass` (`local.Resource_Ref_Local`) (`KismetMathLibrary.Conv_VectorToTransform` _location) "Undefined" "OverrideRootScale" null null))))

(fn `UserConstructionScript`)