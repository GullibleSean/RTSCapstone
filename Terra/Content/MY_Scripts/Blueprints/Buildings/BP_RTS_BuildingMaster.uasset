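; BP_RTS_BuildingMaster is an RTS building actor, apparently a base class, that handles timed construction and its own info HUD.
; Once spawned, it advances a game clock on Tick using game speed from the GameState, completing when scaled work reaches construction time.
; A material swap turns the preview look into the built wall.
; A PlayerController event shows the building's widget when it targets this actor, switching input to UI-only.
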(event `self.ReceiveBeginPlay`
  (`|ExecutionSequence`
    (:`then_0`
      (`self.ReferenceCast`))
    (:`then_1`
      (add `/Game/MY_Scripts/Blueprints/Game_Settings/BP_RTS_GameState.Game_Speed_Control` (`self.GameStateRef`) (`|CreateDelegate` :!event `GetGameSpeed`))
      (bind _game_speed (`/Game/MY_Scripts/Blueprints/Game_Settings/BP_RTS_GameState.Get_Game_Speed` (`self.GameStateRef`)))
      (set `self.GameSpeed` _game_speed))
    (:`then_2`
      (add `/Game/MY_Scripts/Blueprints/Player/BP_RTS_PlayerController.DisplayHUD` (`self.PlayerControllerRef`) (`|CreateDelegate` :!event `DisplayBuildingHUD`)))))

(event `OnSpawn`
  (set `self.IsUnderConstruction` true))

(event `GetGameSpeed`
  (params (GameSpeed :type "Float (double-precision)"))
  (set `self.GameSpeed` GameSpeed))

(event `self.ReceiveTick`
  (params (DeltaSeconds :type "Float (single-precision)"))
  (set `self.DeltaTime` DeltaSeconds)
  (if (and (`self.IsUnderConstruction`) (not (`self.IsBuilt`)))
    (bind _output_get (set `self.GameClock` (`/Game/MY_Scripts/Blueprints/Libraries/BP_RTS_FunctionLib.Set_Game_Time` (`self.DeltaTime`) (`self.GameSpeed`) (`self.GameClock`))))
    (set `self.TimeWorked` (* _output_get (`self.ConstructionModifier`) 60.0))
    (if (>= (`self.TimeWorked`) (`self.ConstructionTime`))
      (set `self.IsBuilt` true)
      (set `self.IsUnderConstruction` false)
      (`PrimitiveComponent.SetMaterial` (`self.BuildingMesh`) 0 "/Game/StarterContent/Materials/M_Basic_Wall.M_Basic_Wall"))))

(event `DisplayBuildingHUD`
  (params (Actor :type "Actor Object Reference") (Bypass :type Boolean))
  (bind _playercontrollerref (`self.PlayerControllerRef`))
  (if (== Actor self)
    (`UserWidget.AddToViewport` (`self.BuildingHUD`) 1)
    (`WidgetBlueprintLibrary.SetInputMode_UIOnlyEx` _playercontrollerref null)
    (`Widget.SetIsEnabled` (`/Game/MY_Scripts/Blueprints/Player/BP_RTS_PlayerController.HUDMainGameRef` _playercontrollerref) true)))

(fn `SetConstructionTime`
  (params (ConstructionTimeRaw :type "Float (double-precision)"))
  (set `self.ConstructionTime` (* ConstructionTimeRaw 60.0))
  (return))

(fn `SetOccupantNames`
  (params (Units :type "Array of /Game/MY_Scripts/Blueprints/Units/BP_RTS_Unit_Master Object Reference (by ref)"))
  (returns (Success :type Boolean))
  (return false))

(fn `UserConstructionScript`
  (`StaticMeshComponent.SetStaticMesh` (`self.BuildingMesh`) (`self.DisplayMesh`))
  (if (`self.IsBuilt`)
    (`PrimitiveComponent.SetMaterial` (`self.BuildingMesh`) 0 "/Game/StarterContent/Materials/M_Basic_Wall.M_Basic_Wall")
    (else
      (`PrimitiveComponent.SetMaterial` (`self.BuildingMesh`) 0 "/Game/MY_Scripts/Materials/Construction/MAT_Preview_Inst.MAT_Preview_Inst"))))