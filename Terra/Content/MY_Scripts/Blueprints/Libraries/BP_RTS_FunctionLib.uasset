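; RTS Blueprint function library with helpers for the game clock and mouse cursor targeting.
; SetGameTime divides delta time by game speed, adds the initial time, and splits the result by 24 into a day count and time of day.
; SetCursorWorldPosition deprojects the mouse from the given controller, line traces up to the sight distance, and returns the hit location when an actor is hit.
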(fn `Set_Cursor_World_Position`
  (params (Controler :type "/Game/MY_Scripts/Blueprints/Player/BP_RTS_PlayerController Object Reference") (Sight_Distance :type "Float (double-precision)"))
  (returns (Relative_Cursor_Ingame :type "Vector Structure"))
  (bind (_worldlocation _worlddirection) (`PlayerController.DeprojectMousePositionToWorld` Controler))
  (bind _outhit (`KismetSystemLibrary.LineTraceSingle` null _worldlocation (+ _worldlocation (* _worlddirection Sight_Distance)) "TraceTypeQuery3"))
  (bind (_bblockinghit _binitialoverlap _time _distance _location _impactpoint _normal _impactnormal _physmat _hitactor) (`GameplayStatics.BreakHitResult` _outhit))
  (if (!= _hitactor null)
    (return _location)))

(fn `Set_Game_Time`
  (params (Delta_Time :type "Float (double-precision)") (Game_Speed :type "Float (double-precision)") (Initial_Game_Time :type "Float (double-precision)"))
  (returns (Game_Time :type "Float (double-precision)") (Day_Count :type Integer))
  (bind (_remainder _returnvalue) (`KismetMathLibrary.FMod` (+ (/ Delta_Time Game_Speed) Initial_Game_Time) 24.0))
  (return _remainder _returnvalue))