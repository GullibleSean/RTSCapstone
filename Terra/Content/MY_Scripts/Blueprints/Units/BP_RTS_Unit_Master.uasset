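; BP_RTS_Unit_Master is the RTS unit master Blueprint, providing selection visuals and shared game references.
; Two functions swap the selected and deselected decals by toggling both visibility and hidden-in-game.
; ReferenceCast caches the RTS game state and player 0's controller through casts.
; DisplayUnitHUD checks that the actor is itself and is either bypassed or not hidden, but then performs no action.
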(event `DisplayUnitHUD`
  (params (Actor :type "Actor Object Reference") (Bypass :type Boolean))
  (if (and (== Actor self) (or Bypass (not (`self.IsHidden`))))
    _))

(fn `Set_Deselected_Decal`
  (bind _deselecteddecal (`self.DeSelectedDecal`))
  (bind _selecteddecal (`self.SelectedDecal`))
  (`SceneComponent.SetVisibility` _selecteddecal false false)
  (`SceneComponent.SetHiddenInGame` _selecteddecal true false)
  (`SceneComponent.SetVisibility` _deselecteddecal true false)
  (`SceneComponent.SetHiddenInGame` _deselecteddecal false false)
  (return))

(fn `Set_Selected_Decal`
  (bind _deselecteddecal (`self.DeSelectedDecal`))
  (bind _selecteddecal (`self.SelectedDecal`))
  (`SceneComponent.SetVisibility` _deselecteddecal false false)
  (`SceneComponent.SetHiddenInGame` _deselecteddecal true false)
  (`SceneComponent.SetVisibility` _selecteddecal true false)
  (`SceneComponent.SetHiddenInGame` _selecteddecal false false)
  (return))

(fn `UserConstructionScript`)