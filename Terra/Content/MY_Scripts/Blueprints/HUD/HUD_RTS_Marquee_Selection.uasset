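; HUD for RTS drag-box unit selection, drawing a translucent green marquee between the clicked and current mouse positions.
; Input start clears the previous selection and records the anchor, hold updates the far corner, and release passes SelectedUnits to BP_RTS_PlayerController.
; While dragging, DrawHUD queries GetActorsInSelectionRectangle for BP_RTS_Unit_Master actors and marks them selected with decals.
; Units accumulate during a drag and are not removed when the box shrinks.
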(event `self.ReceiveBeginPlay`
  (set `self.Controller_Reference` (cast `/Game/MY_Scripts/Blueprints/Player/BP_RTS_PlayerController` (`GameplayStatics.GetPlayerController` 0) :!pure true)))

(event `/Game/MY_Scripts/Blueprints/Libraries/BPI_RTS_Marquee_Selection.On_Input_Start`
  (bind (_locationx _locationy) (`PlayerController.GetMousePosition` (`self.Controller_Reference`)))
  (if (>= (`KismetArrayLibrary.Array_LastIndex` (`self.Selected_Units`)) 0)
    (for _array_element (`self.Selected_Units`)
      (`/Game/MY_Scripts/Blueprints/Units/BP_RTS_Unit_Master.Set_Deselected_Decal` _array_element)
      (set `/Game/MY_Scripts/Blueprints/Units/BP_RTS_Unit_Master.Is_Selected` false _array_element)
      (set `/Game/MY_Scripts/Blueprints/Player/BP_RTS_PlayerController.Is_Unit_Selected` false (`self.Controller_Reference`)))
    (`KismetArrayLibrary.Array_Clear` (`self.Selected_Units`)))
  (bind _output_get (set `self.Clicked_Location` (`KismetMathLibrary.MakeVector2D` _locationx _locationy)))
  (set `self.Holding_Location` _output_get)
  (set `self.Is_Drawing` true))

(event `/Game/MY_Scripts/Blueprints/Libraries/BPI_RTS_Marquee_Selection.On_Input_Release`
  (params (Hold_Time :type "Float (single-precision)"))
  (set `self.Is_Drawing` false)
  (`/Game/MY_Scripts/Blueprints/Player/BP_RTS_PlayerController.Set_Selected_Units` (`self.Controller_Reference`) (`self.Selected_Units`)))

(event `self.ReceiveDrawHUD`
  (params (SizeX :type Integer) (SizeY :type Integer))
  (if (`self.Is_Drawing`)
    (`|ExecutionSequence`
      (:`then_0`
        (`self.Draw_Marquee`)
        (bind _output_get (set `self.Units_In_Selection_Area` (`self.GetActorsInSelectionRectangle` "/Game/MY_Scripts/Blueprints/Units/BP_RTS_Unit_Master.BP_RTS_Unit_Master_C" (`self.Clicked_Location`) (`self.Holding_Location`))))
        (for _array_element _output_get
          (if (`KismetMathLibrary.ClassIsChildOf` (`GameplayStatics.GetObjectClass` _array_element) "/Game/MY_Scripts/Blueprints/Units/BP_RTS_Unit_Master.BP_RTS_Unit_Master_C")
            (bind _asbp_rts_unit_master (cast `/Game/MY_Scripts/Blueprints/Units/BP_RTS_Unit_Master` _array_element))
            (set `self.Selected_Unit` _asbp_rts_unit_master)
            (`|ExecutionSequence`
              (:`then_0`
                (`KismetArrayLibrary.Array_AddUnique` (`self.Selected_Units`) (`self.Selected_Unit`)))
              (:`then_1`
                (for _array_element_2 (`self.Selected_Units`)
                  (`/Game/MY_Scripts/Blueprints/Units/BP_RTS_Unit_Master.Set_Selected_Decal` _array_element_2)
                  (set `/Game/MY_Scripts/Blueprints/Units/BP_RTS_Unit_Master.Is_Selected` true _array_element_2))))))))))

(event `Draw_Marquee`
  (bind _clicked_location (`self.Clicked_Location`))
  (bind (_x _y) (`KismetMathLibrary.BreakVector2D` (`self.Holding_Location`)))
  (bind (_x_2 _y_2) (`KismetMathLibrary.BreakVector2D` _clicked_location))
  (bind (_x_3 _y_3) (`KismetMathLibrary.BreakVector2D` (`self.Clicked_Location`)))
  (bind (_x_4 _y_4) (`KismetMathLibrary.BreakVector2D` (- (`self.Holding_Location`) _clicked_location)))
  (`self.DrawRect` (struct) _x_3 _y_3)
  (`self.DrawRect` (struct) _x _y)
  (`self.DrawRect` (struct :`R` 0.377471 :`G` 0.8125 :`B` 0.428897 :`A` 0.6) _x_2 _y_2 _x_4 _y_4))

(event `/Game/MY_Scripts/Blueprints/Libraries/BPI_RTS_Marquee_Selection.On_Input_Hold`
  (bind (_locationx _locationy) (`PlayerController.GetMousePosition` (`self.Controller_Reference`)))
  (set `self.Holding_Location` (`KismetMathLibrary.MakeVector2D` _locationx _locationy)))

(fn `UserConstructionScript`)