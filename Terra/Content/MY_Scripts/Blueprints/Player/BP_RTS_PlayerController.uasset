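; RTS player controller that handles camera control, unit selection and orders, and building preview placement input.
; Input moves, edge-scrolls, zooms and gate-rotates the camera pawn, with a shared speed modifier for movement.
; Primary click drives the HUD marquee; secondary click sends selected units to the cursor via AIMoveTo with a decal, or cancels building mode's preview.
; BeginPlay spawns the preview actor and main UI; Tick moves the preview to the cursor.
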(event `self.ReceiveBeginPlay`
  (`|ExecutionSequence`
    (:`then_0`
      (`self.ReferenceCast`))
    (:`then_1`
      (bind _returnvalue (`|SpawnActorFromClass` "/Game/MY_Scripts/Blueprints/Buildings/BP_RTS_PreviewBuilding.BP_RTS_PreviewBuilding_C" (`self.EmptyTransform`) "AlwaysSpawn" "OverrideRootScale" null self null))
      (set `self.ContructionPreviewRef` _returnvalue))
    (:`then_2`
      (`self.SpawnWidgets`)
      (`UserWidget.AddToViewport` (`self.HUD_Game_Time_Ref`) 0)
      (`self.Set_HUD_Visibility` "Visible"))
    (:`then_3`
      (`WidgetBlueprintLibrary.SetInputMode_GameAndUIEx` self null))))

(event `self.ReceiveTick`
  (params (DeltaSeconds :type "Float (single-precision)"))
  (set `self.Delta_Time` DeltaSeconds)
  (if (`self.Is_Holding_Input`)
    (`self.Update_Selection`)
    (elif (and (`self.Is_Building_Mode_Active`) (!= (`self.ContructionPreviewRef`) null))
      (`/Game/MY_Scripts/Blueprints/Buildings/BP_RTS_PreviewBuilding.GetCursorPosition` (`self.ContructionPreviewRef`) (`/Game/MY_Scripts/Blueprints/Libraries/BP_RTS_FunctionLib.Set_Cursor_World_Position` self 10000.0)))))

(event `InputAction|SpeedModifier`
  (params (Key :type "Key Structure"))
  ;[0.1529 0.107 0.4072] Movement Controls
  ;;[1 1 1] Set Movement Speed Modifier
  (:`Pressed`
    (set `self.Movement_Speed_modifier` 1.5))
  (:`Released`
    (set `self.Movement_Speed_modifier` 1.0)))

(event `InputAxis|MoveForward`
  (params (AxisValue :type "Float (single-precision)"))
  ;[0.1529 0.107 0.4072] Movement Controls
  ;;[1 1 1] Basic Movement Controls
  (if (not (`self.Disable_Pan_Movement`))
    (`self.BasicMovementControls` AxisValue (stale `InputAxis|MoveRight` AxisValue) :!label _label)))

(event `InputAction|ZoomIn`
  (params (Key :type "Key Structure"))
  (bind _cameraboom (`/Game/MY_Scripts/Blueprints/Player/BP_RTS_CameraPawn.CameraBoom` (`self.Camera_Pawn_Ref`)))
  ;[0.3782 0.2648 1] Zoom Control
  ;;[1 1 1] Zoom In
  (:`Pressed`
    (set `SpringArmComponent.TargetArmLength` (`KismetMathLibrary.FClamp` (- (`SpringArmComponent.TargetArmLength` _cameraboom) (`self.Cam_Zoom_Speed`)) (`self.Min_Zoom_Limit`) (`self.Max_Zoom_Limit`)) _cameraboom)))

(event `InputAction|ZoomReset`
  (params (Key :type "Key Structure"))
  ;[0.3782 0.2648 1] Zoom Control
  ;;[1 1 1] Reset Zoom
  (:`Pressed`
    (set `SpringArmComponent.TargetArmLength` (`self.Default_Arm_Length`) (`/Game/MY_Scripts/Blueprints/Player/BP_RTS_CameraPawn.CameraBoom` (`self.Camera_Pawn_Ref`)))))

(event `InputAxis|MoveRight`
  (params (AxisValue :type "Float (single-precision)"))
  ;[0.1529 0.107 0.4072] Movement Controls
  ;;[1 1 1] Basic Movement Controls
  (if (not (`self.Disable_Pan_Movement`))
    (goto _label :!via `Right Movement`)))

(event `InputAxisKey|MouseX`
  (params (AxisValue :type "Float (single-precision)"))
  ;[0.1529 0.107 0.4072] Movement Controls
  ;;[1 1 1] Edge Scroll Movement
  (if (not (`self.Disable_Camera_Movement`))
    (bind (_deltaspeedx _deltaspeedy) (`self.EdgeScroll` :!label _label_2))
    (`self.K2_AddActorLocalOffset` (`self.Camera_Pawn_Ref`) (`KismetMathLibrary.MakeVector` _deltaspeedx _deltaspeedy) true false)))

(event `InputAxisKey|MouseY`
  (params (AxisValue :type "Float (single-precision)"))
  ;[0.1529 0.107 0.4072] Movement Controls
  ;;[1 1 1] Edge Scroll Movement
  (if (not (`self.Disable_Camera_Movement`))
    (goto _label_2 :!via `MouseY`)))

(event `InputAction|ZoomOut`
  (params (Key :type "Key Structure"))
  (bind _cameraboom (`/Game/MY_Scripts/Blueprints/Player/BP_RTS_CameraPawn.CameraBoom` (`self.Camera_Pawn_Ref`)))
  ;[0.3782 0.2648 1] Zoom Control
  ;;[1 1 1] Zoom Out
  (:`Pressed`
    (set `SpringArmComponent.TargetArmLength` (`KismetMathLibrary.FClamp` (+ (`self.Cam_Zoom_Speed`) (`SpringArmComponent.TargetArmLength` _cameraboom)) (`self.Min_Zoom_Limit`) (`self.Max_Zoom_Limit`)) _cameraboom)))

(event `Key|V`
  (params (Key :type "Key Structure"))
  (bind (_relative_cursor_ingame_x _relative_cursor_ingame_y) (`KismetMathLibrary.BreakVector` (`/Game/MY_Scripts/Blueprints/Libraries/BP_RTS_FunctionLib.Set_Cursor_World_Position` self 10000.0)))
  ;[1 1 1] For Testing Only (will delete later)
  (:`Pressed`
    (`|SpawnActorFromClass` "/Game/MY_Scripts/Blueprints/Units/BP_RTS_Unit_Master.BP_RTS_Unit_Master_C" (`KismetMathLibrary.MakeTransform` (`KismetMathLibrary.MakeVector` _relative_cursor_ingame_x _relative_cursor_ingame_y 150.0)) "Undefined" "OverrideRootScale" null null)))

(event `InputAction|PanReset`
  (params (Key :type "Key Structure"))
  (bind _camera_pawn_ref (`self.Camera_Pawn_Ref`))
  ;[0.1529 0.107 0.4072] Pan Control
  ;;[1 1 1] Reset Camera Pan
  (:`Pressed`
    (`self.K2_SetActorRotation` _camera_pawn_ref (`KismetMathLibrary.MakeRotator` (.roll (`self.K2_GetActorRotation` _camera_pawn_ref)) 0.0 (.yaw (`self.K2_GetActorRotation` _camera_pawn_ref))) false)))

(event `InputAction|Pan`
  (params (Key :type "Key Structure"))
  (bind _camera_pawn_ref (`self.Camera_Pawn_Ref`))
  ;[0.1529 0.107 0.4072] Pan Control
  ;;[1 1 1] Pan X
  (:`Pressed`
    (set `self.Disable_Pan_Movement` true)
    (goto _label_3 :!via `Open`))
  (:`Released`
    (set `self.Disable_Pan_Movement` false)
    (goto _label_3 :!via `Close`)))

(event `InputAxisKey|MouseX`
  (params (AxisValue :type "Float (single-precision)"))
  (bind _camera_pawn_ref (`self.Camera_Pawn_Ref`))
  ;[0.1529 0.107 0.4072] Pan Control
  ;;[1 1 1] Pan X
  (`/Engine/EditorBlueprintResources/StandardMacros.Gate` true :!label _label_3
    (:`Exit`
      (`self.K2_SetActorRotation` _camera_pawn_ref (`KismetMathLibrary.MakeRotator` (.roll (`self.K2_GetActorRotation` _camera_pawn_ref)) (.pitch (`self.K2_GetActorRotation` _camera_pawn_ref)) (+ (.yaw (`self.K2_GetActorRotation` _camera_pawn_ref)) (* AxisValue (`self.Pan_Speed`)))) false))))

(event `InputAction|RotatePreviewLeft`
  (params (Key :type "Key Structure"))
  (bind _contructionpreviewref (`self.ContructionPreviewRef`))
  (bind (_returnvalue_roll _returnvalue_pitch _returnvalue_yaw) (`KismetMathLibrary.BreakRotator` (`self.K2_GetActorRotation` _contructionpreviewref)))
  (:`Pressed`
    (set `self.Disable_Camera_Movement` true)
    (if (and (`self.Is_Building_Mode_Active`) (!= _contructionpreviewref null))
      (`self.K2_SetActorRotation` _contructionpreviewref (`KismetMathLibrary.MakeRotator` _returnvalue_roll _returnvalue_pitch (+ _returnvalue_yaw (`self.ConstractionRotationRate`))) false)))
  (:`Released`
    (set `self.Disable_Camera_Movement` false)))

(event `InputAction|Pan`
  (params (Key :type "Key Structure"))
  (bind _camera_pawn_ref (`self.Camera_Pawn_Ref`))
  ;[0.1529 0.107 0.4072] Pan Control
  ;;[1 1 1] Pan Y
  (:`Pressed`
    (set `self.Disable_Pan_Movement` true)
    (goto _label_4 :!via `Open`))
  (:`Released`
    (set `self.Disable_Pan_Movement` false)
    (goto _label_4 :!via `Close`)))

(event `InputAxisKey|MouseY`
  (params (AxisValue :type "Float (single-precision)"))
  (bind _camera_pawn_ref (`self.Camera_Pawn_Ref`))
  ;[0.1529 0.107 0.4072] Pan Control
  ;;[1 1 1] Pan Y
  (`/Engine/EditorBlueprintResources/StandardMacros.Gate` true :!label _label_4
    (:`Exit`
      (`self.K2_SetActorRotation` _camera_pawn_ref (`KismetMathLibrary.MakeRotator` (.roll (`self.K2_GetActorRotation` _camera_pawn_ref)) (`KismetMathLibrary.FClamp` (+ (.pitch (`self.K2_GetActorRotation` _camera_pawn_ref)) (* AxisValue (`self.Pan_Speed`))) -25.0 45.0) (.yaw (`self.K2_GetActorRotation` _camera_pawn_ref))) false))))

(event `InputAction|RotatePreviewRight`
  (params (Key :type "Key Structure"))
  (bind _contructionpreviewref (`self.ContructionPreviewRef`))
  (bind (_returnvalue_roll _returnvalue_pitch _returnvalue_yaw) (`KismetMathLibrary.BreakRotator` (`self.K2_GetActorRotation` _contructionpreviewref)))
  (:`Pressed`
    (set `self.Disable_Camera_Movement` true)
    (if (and (`self.Is_Building_Mode_Active`) (!= _contructionpreviewref null))
      (`self.K2_SetActorRotation` _contructionpreviewref (`KismetMathLibrary.MakeRotator` _returnvalue_roll _returnvalue_pitch (- _returnvalue_yaw (`self.ConstractionRotationRate`))) false)))
  (:`Released`
    (set `self.Disable_Camera_Movement` false)))

(event `InputAction|PrimaryAction`
  (params (Key :type "Key Structure"))
  ;[1 1 1] Draw Marquee on Press and Release
  (:`Pressed`
    (if (not (`self.Is_Building_Mode_Active`))
      (message `/Game/MY_Scripts/Blueprints/Libraries/BPI_RTS_Marquee_Selection.On_Input_Start` (`self.Marquee_Ref`))
      (set `self.Holding_Time` 0.0)
      (set `self.Is_Holding_Input` true)))
  (:`Released`
    (if (not (`self.Is_Building_Mode_Active`))
      (message `/Game/MY_Scripts/Blueprints/Libraries/BPI_RTS_Marquee_Selection.On_Input_Release` (`self.Marquee_Ref`) (`self.Holding_Time`))
      (set `self.Is_Holding_Input` false))))

(event `Update_Selection`
  ;[1 1 1] Draw Marquee on Press and Release
  (if (`self.Is_Holding_Input`)
    (set `self.Holding_Time` (+ (`self.Holding_Time`) (`self.Delta_Time`)))
    (message `/Game/MY_Scripts/Blueprints/Libraries/BPI_RTS_Marquee_Selection.On_Input_Hold` (`self.Marquee_Ref`))))

(event `InputAction|SecondaryAction`
  (params (Key :type "Key Structure"))
  (bind (_hitresult _returnvalue) (`self.GetHitResultUnderCursorByChannel` "TraceTypeQuery1" false))
  (bind _previous_location_decal (`self.Previous_Location_Decal`))
  (bind _previous_location_decal_2 (`self.Previous_Location_Decal`))
  (:`Pressed`
    (if (`self.Is_Building_Mode_Active`)
      (`/Game/MY_Scripts/Blueprints/Buildings/BP_RTS_PreviewBuilding.DestroyPreview` (`self.ContructionPreviewRef`))
      (elif (`self.Is_Unit_Selected`)
        (if _returnvalue
          (set `self.Target_Location` (`.Location` (`GameplayStatics.BreakHitResult` _hitresult)))
          (`|ExecutionSequence`
            (:`then_0`
              (`/Engine/EditorBlueprintResources/StandardMacros.IsValid` _previous_location_decal_2
                (:`Is Valid`
                  (`ActorComponent.K2_DestroyComponent` _previous_location_decal_2)
                  (bind _returnvalue_2 (`AIBlueprintHelperLibrary.GetAIController` (stale _array_element)))
                  (`self.StopMovement` _returnvalue_2))
                (:`Is Not Valid`
                  _))
              (bind _returnvalue_3 (`GameplayStatics.SpawnDecalAtLocation` "/Game/MY_Scripts/Materials/Movement_Selection_Decal.Movement_Selection_Decal" (32.0 64.0 64.0) (`self.Target_Location`)))
              (set `self.Previous_Location_Decal` _returnvalue_3))
            (:`then_1`
              (for _array_element (`self.Selected_Units`)
                (`self.StopMovement` _returnvalue_2)
                (`AITask_MoveTo.AIMoveTo` _returnvalue_2 (`self.Target_Location`) null -1.0 "Disable" "Enable" true false
                  (:`OnMoveFinished`
                    (`/Engine/EditorBlueprintResources/StandardMacros.IsValid` _previous_location_decal
                      (:`Is Valid`
                        (`ActorComponent.K2_DestroyComponent` _previous_location_decal)))))))))))))

(fn `Set_HUD_Visibility`
  (params (Game_Time_HUD :type "ESlateVisibility Enum" :default "Visible"))
  (`Widget.SetVisibility` (`self.HUD_Game_Time_Ref`) Game_Time_HUD))

(fn `Set_Selected_Units`
  (params (Selected_Units :type "Array of /Game/MY_Scripts/Blueprints/Units/BP_RTS_Unit_Master Object Reference"))
  (set `self.Selected_Units` Selected_Units)
  (if (>= (`KismetArrayLibrary.Array_LastIndex` (`self.Selected_Units`)) 0)
    (set `self.Is_Unit_Selected` true)))

(fn `SetBuildingModeActive`
  (params (IsActive :type Boolean))
  (set `self.Is_Building_Mode_Active` IsActive)
  (return))

(fn `UserConstructionScript`)